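; Box1 is a package actor that plays a sound when clicked and can be opened to reveal its contents.
; The OpenPackage input, guarded to run once, plays an opening sound, fades the player character and ends its inspection state.
; After a short delay it spawns a polaroid, letter, bear and box at hard-coded world transforms, resets inspection again and destroys itself.
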(event `self.ReceiveActorOnClicked`
  (params (ButtonPressed :type "Key Structure"))
  (`GameplayStatics.PlaySound2D` "/Game/Assets/Sounds/box.box" 1.25 1.0 0.0 null null))

(event `EnhancedInput|/Game/Input/Actions/OpenPackage`
  (params (ActionValue :type Boolean) (ElapsedSeconds :type "Float (double-precision)") (TriggeredSeconds :type "Float (double-precision)") (InputAction :type "InputAction Object Reference" :default "/Game/Input/Actions/OpenPackage.OpenPackage"))
  (:`Triggered`
    (if (not (`self.bIsOpening`))
      (set `self.bIsOpening` true)
      (`GameplayStatics.PlaySound2D` "/Game/Assets/Sounds/openingpackage.openingpackage" 1.0 1.0 0.0 null null)
      (bind _asbp_third_person_character (cast `/Game/Blueprints/BP_ThirdPersonCharacter` (`GameplayStatics.GetPlayerCharacter` 0)))
      (`/Game/Blueprints/BP_ThirdPersonCharacter.FadeIn` _asbp_third_person_character true)
      (set `/Game/Blueprints/BP_ThirdPersonCharacter.bIsInspecting` false _asbp_third_person_character)
      (`/Game/Blueprints/BP_ThirdPersonCharacter.Reset DoOnce` _asbp_third_person_character)
      (`self.SpawnContent`))))

(event `SpawnContent`
  (`KismetSystemLibrary.Delay` 2.5)
  (`|SpawnActorFromClass` "/Game/Blueprints/ContentPolaroid.ContentPolaroid_C" (`KismetMathLibrary.MakeTransform` (724.0 1203.0 97.148287) (struct :`Pitch` 90.0 :`Yaw` -172.8749 :`Roll` -152.874984)) "Undefined" "MultiplyWithRoot" null null)
  (`|SpawnActorFromClass` "/Game/Blueprints/ContentLetter1.ContentLetter1_C" (`KismetMathLibrary.MakeTransform` (702.9979 1173.5721 86.44893) (struct :`Yaw` 10.0)) "Undefined" "MultiplyWithRoot" null null)
  (`|SpawnActorFromClass` "/Game/Blueprints/ContentBear.ContentBear_C" (`KismetMathLibrary.MakeTransform` (691.0 1206.109661 100.66143) (struct :`Yaw` -40.0)) "Undefined" "MultiplyWithRoot" null null)
  (`|SpawnActorFromClass` "/Game/Blueprints/ContentBox.ContentBox_C" (`KismetMathLibrary.MakeTransform` (686.806645 1124.770507 110.454182) (struct :`Pitch` -90.0 :`Yaw` 90.0 :`Roll` -25.0)) "Undefined" "MultiplyWithRoot" null null)
  (bind _asbp_third_person_character (cast `/Game/Blueprints/BP_ThirdPersonCharacter` (`GameplayStatics.GetPlayerCharacter` 0)))
  (set `/Game/Blueprints/BP_ThirdPersonCharacter.bIsInspecting` false _asbp_third_person_character)
  (`/Game/Blueprints/BP_ThirdPersonCharacter.Reset DoOnce` _asbp_third_person_character)
  (`self.K2_DestroyActor`))

(fn `UserConstructionScript`
  (`parent.UserConstructionScript`))