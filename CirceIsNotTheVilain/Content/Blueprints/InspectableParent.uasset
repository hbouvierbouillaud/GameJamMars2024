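; Base Blueprint for inspectable objects that the player can rotate and click.
; StartInspect moves player input from the Inspector actor to this object.
; While the right mouse button is held, mouse X and Y axes apply yaw and pitch to the MeshPivot.
; A click notifies BP_ThirdPersonCharacter through InteractableObjectClicked, then hands input back to the Inspector.
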(event `Start Inspect`
  (params (Inspector :type "Pawn Object Reference"))
  (bind _returnvalue (`GameplayStatics.GetPlayerController` 0))
  (`self.DisableInput` Inspector _returnvalue)
  (`self.EnableInput` _returnvalue))

(event `self.ReceiveBeginPlay`
  (set `self.Player` null)
  (add `self.OnClicked` (delegate `OnClicked_Event`)))

(event `OnClicked_Event` :!signature `self.OnClicked`
  (params (TouchedActor :type "Actor Object Reference") (ButtonPressed :type "Key Structure" :default "None"))
  (bind _returnvalue (`GameplayStatics.GetPlayerController` 0))
  (bind _asbp_third_person_character (cast `/Game/Blueprints/BP_ThirdPersonCharacter` (`GameplayStatics.GetPlayerCharacter` 0)))
  (`/Game/Blueprints/BP_ThirdPersonCharacter.InteractableObjectClicked` _asbp_third_person_character TouchedActor)
  (`self.DisableInput` _returnvalue)
  (`self.EnableInput` (stale `Start Inspect` Inspector) _returnvalue))

(event `InputAxisKey|MouseX`
  (params (AxisValue :type "Float (single-precision)"))
  (if (`PlayerController.IsInputKeyDown` (`GameplayStatics.GetPlayerController` 0) "RightMouseButton")
    (`SceneComponent.K2_SetRelativeRotation` (`self.MeshPivot`) (`KismetMathLibrary.ComposeRotators` (`SceneComponent.RelativeRotation` (`self.MeshPivot`)) (`KismetMathLibrary.MakeRotator` 0.0 0.0 (* AxisValue -3.0))) false false)))

(event `InputAxisKey|MouseY`
  (params (AxisValue :type "Float (single-precision)"))
  (if (`PlayerController.IsInputKeyDown` (`GameplayStatics.GetPlayerController` 0) "RightMouseButton")
    (`SceneComponent.K2_SetRelativeRotation` (`self.MeshPivot`) (`KismetMathLibrary.ComposeRotators` (`SceneComponent.RelativeRotation` (`self.MeshPivot`)) (`KismetMathLibrary.MakeRotator` 0.0 (* AxisValue -4.0))) false false)))

(fn `UserConstructionScript`)